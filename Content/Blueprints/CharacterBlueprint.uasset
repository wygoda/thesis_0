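; Character Blueprint that moves via input axes and aims a Cylinder component independently with mouse or gamepad, twin-stick style.
; MoveForward and MoveRight feed movement input.
; When MouseRotating is set, Tick eases the cylinder's yaw toward the cursor's visibility-trace hit.
; LookUp and LookRight share logic that eases the same stored Direction toward the stick vector beyond a small dead zone, using RInterpTo with fixed time steps.
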(event EventBeginPlay)

(event Collision|EventActorBeginOverlap
  (params (OtherActor :type Actor%20Object%20Reference)))

(event EventTick
  (params (DeltaSeconds :type Float%20%28single-precision%29))
  ;[1 1 1] Rotating with mouse
  (if (Variables|Default|GetMouseRotating)
    (bind _output_get (Variables|Default|SetDirection (Math|Interpolation|RInterpTo (Variables|Default|GetDirection) (Math|Rotator|MakeRotator 0.0 0.0 (.Yaw (Math|Rotator|BreakRotator (Math|Rotator|FindLookatRotation (Transformation|GetActorLocation) (.Location (Collision|BreakHitResult (.HitResult (Game|Player|GetHitResultUnderCursorbyChannel (Game|GetPlayerController 0) "TraceTypeQuery1" true)))))))) 0.5 0.3)))
    (Transformation|SetWorldRotation (Variables|Default|GetCylinder) _output_get false false)))

(event Input|AxisEvents|InputAxisMoveForward
  (params (AxisValue :type Float%20%28single-precision%29))
  ;[1 1 1] Walking
  (Pawn|Input|AddMovementInput (Math|Vector|MakeVector AxisValue (stale Input|AxisEvents|InputAxisMoveRight AxisValue) 0.0) (Math|Float|Absolute(Float) AxisValue) false))

(event Input|AxisEvents|InputAxisMoveRight
  (params (AxisValue :type Float%20%28single-precision%29))
  ;[1 1 1] Walking
  (Pawn|Input|AddMovementInput (Math|Vector|MakeVector (stale Input|AxisEvents|InputAxisMoveForward AxisValue) AxisValue 0.0) (Math|Float|Absolute(Float) AxisValue) false))

(event Input|AxisEvents|InputAxisLookUp
  (params (AxisValue :type Float%20%28single-precision%29))
  ;[1 1 1] Rotating with gamepad
  (if (> (Math|Vector|VectorLength (Math|Vector|MakeVector AxisValue (stale Input|AxisEvents|InputAxisLookRight AxisValue) 0.0)) 0.1)
    (bind _output_get (Variables|Default|SetDirection (Math|Interpolation|RInterpTo (Variables|Default|GetDirection) (Math|Conversions|RotationFromXVector (Math|Vector|MakeVector AxisValue (stale Input|AxisEvents|InputAxisLookRight AxisValue) 0.0)) 0.5 0.1)))
    (Transformation|SetWorldRotation (Variables|Default|GetCylinder) _output_get false false)))

(event Input|AxisEvents|InputAxisLookRight
  (params (AxisValue :type Float%20%28single-precision%29))
  ;[1 1 1] Rotating with gamepad
  (if (> (Math|Vector|VectorLength (Math|Vector|MakeVector (stale Input|AxisEvents|InputAxisLookUp AxisValue) AxisValue 0.0)) 0.1)
    (bind _output_get (Variables|Default|SetDirection (Math|Interpolation|RInterpTo (Variables|Default|GetDirection) (Math|Conversions|RotationFromXVector (Math|Vector|MakeVector (stale Input|AxisEvents|InputAxisLookUp AxisValue) AxisValue 0.0)) 0.5 0.1)))
    (Transformation|SetWorldRotation (Variables|Default|GetCylinder) _output_get false false)))

(fn ConstructionScript)